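; GA_Ejemplo1 is an example Gameplay Ability for a short-range frontal attack by the avatar.
; On activation it plays a montage at a rate read from a gameplay attribute on the avatar's CustomAbilitySystemComponent.
; The montage's notify spawns an effect system and runs a box trace just ahead of the avatar, applying a gameplay effect to hit actors with that component.
; The graph never commits or ends the ability.
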(event Ability|EventActivateAbility
  (bind _returnvalue (Ability|GetAvatarActorfromActorInfo))
  (bind _returnvalue_2 (Ability|GetAvatarActorfromActorInfo))
  (bind _returnvalue_3 (Transformation|GetActorLocation _returnvalue))
  (bind _returnvalue_4 (Transformation|GetActorRotation _returnvalue))
  (bind _returnvalue_5 (Math|Vector|GetForwardVector _returnvalue_4))
  (bind _returnvalue_6 (* _returnvalue_5 2e+01))
  (bind _returnvalue_7 (+ _returnvalue_3 _returnvalue_6))
  (Animation|Montage|PlayMontage (Actor|GetComponentbyClass _returnvalue_2 "/Script/Engine.SkeletalMeshComponent") 0 (.ReturnValue (Class|AbilitySystemComponent|GetGameplayAttributeValue (Actor|GetComponentbyClass _returnvalue_2 "/Script/UTHUB_GAS.CustomAbilitySystemComponent") "(AttributeName=\"AttackSpeed\",Attribute=/Script/UTHUB_GAS.CoreAttributeSet:AttackSpeed,AttributeOwner=\"/Script/CoreUObject.Class'/Script/UTHUB_GAS.CoreAttributeSet'\")"))
    (:OnNotifyBegin
      (Niagara|SpawnSystematLocation 0 _returnvalue_7 _returnvalue_4)
      (bind _outhits (Class|KismetSystemLibrary|BoxTraceMultibyProfile _returnvalue_7 (+ _returnvalue_6 _returnvalue_7) "30.000000,30.000000,30.000000" _returnvalue_4 "None" false (Utilities|Array|MakeArray (Ability|GetAvatarActorfromActorInfo)) "None" true))
      (for _array_element _outhits
        (Utilities|IsValid (.HitActor (Collision|BreakHitResult _array_element))
          (:Is%20Valid
            (Utilities|IsValid (Actor|GetComponentbyClass (.HitActor (Collision|BreakHitResult _array_element)) "/Script/UTHUB_GAS.CustomAbilitySystemComponent")
              (:Is%20Valid
                (Class|CustomAbilitySystemComponent|ApplyGameplayEffect (Actor|GetComponentbyClass (.HitActor (Collision|BreakHitResult _array_element)) "/Script/UTHUB_GAS.CustomAbilitySystemComponent") (Variables|Default|GetEffect%20Class))))))))))

(event Ability|EventOnEndAbility
  (params (bWasCancelled :type Boolean)))