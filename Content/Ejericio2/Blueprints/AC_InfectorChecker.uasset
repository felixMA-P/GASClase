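; AC_InfectorChecker is an actor component that lets an infected owner apply gameplay effects to nearby pawns.
; A looping timer started on BeginPlay checks whether the owner's ability system component has the Gameplay.Infection.Infected tag.
; If so, a sphere overlap around the owner finds other pawns and applies every effect in Effectors to those with a CustomAbilitySystemComponent.
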(event Custom|CheckOverlapping
  (if (GameplayTags|HasTag (GameplayTags|GetOwnedGameplayTags (Actor|GetComponentbyClass (Components|GetOwner) "/Script/UTHUB_GAS.CustomAbilitySystemComponent") :!class /Script/GameplayTags.GameplayTagAssetInterface) "(TagName=\"Gameplay.Infection.Infected\")")
    (bind _outactors (Collision|SphereOverlapActors (Transformation|GetActorLocation (Components|GetOwner)) (Variables|Default|GetSphere%20Radius) (Utilities|Array|MakeArray "ObjectTypeQuery3") 0 (Utilities|Array|MakeArray (Components|GetOwner))))
    (for _array_element _outactors
      (Utilities|IsValid (Actor|GetComponentbyClass _array_element "/Script/UTHUB_GAS.CustomAbilitySystemComponent")
        (:Is%20Valid
          (for _array_element_2 (Variables|Default|GetEffectors)
            (Class|CustomAbilitySystemComponent|ApplyGameplayEffect (Actor|GetComponentbyClass _array_element "/Script/UTHUB_GAS.CustomAbilitySystemComponent") _array_element_2)))))))

(event EventBeginPlay
  (Utilities|Time|SetTimerbyEvent (delegate Custom|CheckOverlapping) (Variables|Default|GetFrecuency) true))

(event EventTick
  (params (DeltaSeconds :type Float%20%28single-precision%29)))