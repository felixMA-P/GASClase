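; Gameplay ability for the mage character that casts a timed arcane shield.
; On activation it plays the CastSpell montage, and on completion attaches the N_ArcaneShield Niagara system to the avatar's skeletal mesh.
; It then applies a gameplay effect through the avatar's CustomAbilitySystemComponent and ends after a fixed delay, destroying the Niagara component in OnEndAbility.
; Only montage completion is handled, and EndAbility runs only when that component is valid.
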(event Ability|EventActivateAbility
  (bind _returnvalue (Ability|GetAvatarActorfromActorInfo))
  (bind _returnvalue_2 (Actor|GetComponentbyClass _returnvalue "/Script/UTHUB_GAS.CustomAbilitySystemComponent"))
  (Utilities|PlayCustomMontage (Ability|GetAvatarActorfromActorInfo) "/Game/MageCharacter/Animations/CastSpell.CastSpell"
    (:On%20Completed
      (bind _returnvalue_3 (Niagara|SpawnSystemAttached "/Game/MegaMagicVFXBundle/VFX/MagicShieldsVFX/VFX/DefaultVersions/ArcaneShield/Systems/N_ArcaneShield.N_ArcaneShield" (Actor|GetComponentbyClass (Ability|GetAvatarActorfromActorInfo) "/Script/Engine.SkeletalMeshComponent") "None" "0, 0, 0" "0, 0, 0" "SnapToTarget" false))
      (Variables|Default|SetSystem _returnvalue_3)
      (Utilities|IsValid _returnvalue
        (:Is%20Valid
          (Utilities|IsValid _returnvalue_2
            (:Is%20Valid
              (Class|CustomAbilitySystemComponent|ApplyGameplayEffect _returnvalue_2 (Variables|Default|GetGameplaytEffect))
              (Utilities|FlowControl|Delay 1e+01)
              (Ability|EndAbility))))))))

(event Ability|EventOnEndAbility
  (params (bWasCancelled :type Boolean))
  (Components|DestroyComponent (Variables|Default|GetSystem)))