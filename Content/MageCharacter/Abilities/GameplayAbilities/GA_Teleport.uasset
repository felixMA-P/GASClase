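; Mage gameplay ability that teleports the avatar to the point under player 0's cursor.
; It spawns blackhole explosion effects at origin and destination, issues a SimpleMoveToLocation, then sets the actor's location after a brief delay and later destroys both effects.
; The destination adds the avatar's current Z to the hit Z, and the cursor trace re-runs after the delay.
; The graph never commits or ends the ability.
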(event Ability|EventActivateAbility
  (bind _returnvalue (Ability|GetAvatarActorfromActorInfo))
  (bind _returnvalue_2 (Game|GetPlayerController 0))
  (bind _hitresult (Game|Player|GetHitResultUnderCursorbyChannel _returnvalue_2 "TraceTypeQuery1" true))
  (bind _returnvalue_3 (Transformation|GetActorLocation _returnvalue))
  (bind _location (Collision|BreakHitResult _hitresult))
  (bind (_x _y _z) (Math|Vector|BreakVector _location))
  (bind _returnvalue_4 (+ _z (.z _returnvalue_3)))
  (bind _returnvalue_5 (Math|Vector|MakeVector _x _y _returnvalue_4))
  (bind _returnvalue_6 (Niagara|SpawnSystematLocation "/Game/MegaMagicVFXBundle/VFX/MagicalExplosionsVFX/VFX/BlackholeExplosion/Systems/N_BlackholeExplosion.N_BlackholeExplosion" _returnvalue_5))
  (bind _returnvalue_7 (Niagara|SpawnSystematLocation "/Game/MegaMagicVFXBundle/VFX/MagicalExplosionsVFX/VFX/BlackholeExplosion/Systems/N_BlackholeExplosion.N_BlackholeExplosion" (Transformation|GetActorLocation _returnvalue)))
  (AI|Navigation|SimpleMovetoLocation (Game|GetPlayerController 0) _returnvalue_5)
  (Utilities|FlowControl|Delay 0.1)
  (Transformation|SetActorLocation _returnvalue _returnvalue_5 false false)
  (Utilities|FlowControl|Delay 0.5)
  (Components|Activation|Deactivate _returnvalue_6)
  (Components|DestroyComponent _returnvalue_6)
  (Components|Activation|Deactivate _returnvalue_7)
  (Components|DestroyComponent _returnvalue_7))

(event Ability|EventOnEndAbility
  (params (bWasCancelled :type Boolean)))